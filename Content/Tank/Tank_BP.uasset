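; Player tank pawn Blueprint that wires movement, aiming, camera and health bar together.
; On BeginPlay it hands the tracks to the TankMovement component, the barrel and turret to Aiming, and itself to the health bar widget.
; Input forwards throttle and move axes to TankMovement and fire to Aiming.
; Aim axes rotate an azimuth gimbal and spring arm, and SwapCamera toggles first- and third-person cameras.
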(event EventBeginPlay
  (Class|TankMovementComponent|Initialise (Variables|Default|GetTankMovement) (Variables|Default|GetLeftTrack) (Variables|Default|GetRightTrack))
  (Class|AimingComponent|Initialise (Variables|Default|GetAiming) (Variables|Default|GetBarrel) (Variables|Default|GetTurret))
  (CallFunction|InitialiseHealthbarWidget))

(event Input|ActionEvents|InputActionFire
  (params (Key :type Key%20Structure :default "None"))
  (:Pressed
    (Class|AimingComponent|Fire (Variables|Default|GetAiming))))

(event Input|ActionEvents|InputActionSwapCamera
  (params (Key :type Key%20Structure :default "None"))
  (:Pressed
    (Components|Activation|ToggleActive (Variables|Default|Get1st%20Person))
    (Components|Activation|ToggleActive (Variables|Default|Get3rd%20Person))))

(event Input|AxisEvents|InputAxisAimAzimuth
  (params (AxisValue :type Float%20%28single-precision%29))
  (Transformation|AddLocalRotation (Variables|Default|GetAzimuth%20Gimbal) (Math|Rotator|MakeRotator 0.0 0.0 AxisValue) false false))

(event Input|AxisEvents|InputAxisAimElevation
  (params (AxisValue :type Float%20%28single-precision%29))
  (Transformation|AddLocalRotation (Variables|Default|GetSpringArm) (Math|Rotator|MakeRotator 0.0 AxisValue 0.0) false false))

(event Input|AxisEvents|InputAxisBackward
  (params (AxisValue :type Float%20%28single-precision%29))
  (Class|TankMovementComponent|IntendMoveForward (Variables|Default|GetTankMovement) AxisValue))

(event Input|AxisEvents|InputAxisLeftThrottle
  (params (AxisValue :type Float%20%28single-precision%29))
  (Class|TankMovementComponent|IntendTurnLeft (Variables|Default|GetTankMovement) AxisValue))

(event Input|AxisEvents|InputAxisRightThrottle
  (params (AxisValue :type Float%20%28single-precision%29))
  (Class|TankMovementComponent|IntendTurnRight (Variables|Default|GetTankMovement) AxisValue))

(event Input|AxisEvents|InputAxisForward
  (params (AxisValue :type Float%20%28single-precision%29))
  (Class|TankMovementComponent|IntendMoveForward (Variables|Default|GetTankMovement) AxisValue))

(fn ConstructionScript)

(fn InitialiseHealthbarWidget
  (bind _ashealth_bar (Utilities|Casting|CastToHealthBar (UserInterface|GetUserWidgetObject (Variables|Default|GetHealth%20Bar))))
  (Variables|/Game/Assets/UI/HealthBar.HealthBar_C|SetCurrentTank _ashealth_bar self))